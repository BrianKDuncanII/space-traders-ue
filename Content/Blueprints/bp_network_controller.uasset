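; Network controller actor that checks whether the SpaceTraders API server is reachable at game start and shows the result on screen.
; On BeginPlay it creates a NetworkStats widget and sends a GET request to the API root, setting the status text to connecting, online or offline.
; On success it also shows the server version from the JSON response and opens the agent registration widget if the camera controller is player-controlled.
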(event EventBeginPlay
  (bind _returnvalue (UserInterface|CreateWidget "/Game/Widgets/networkStats.networkStats_C"))
  (UserInterface|Viewport|AddtoViewport _returnvalue 0)
  (Variables|Default|SetNetworkStatsWidget _returnvalue)
  (bind _result_body (|HttpRequest "https://api.spacetraders.io/v2" "Get")
    (:then
      (Variables|/Script/UMG.TextBlock|SetText (Variables|/Game/Widgets/networkStats.networkStats_C|Gettxt_server_status (Variables|Default|GetNetworkStatsWidget)) "Connecting..."))
    (:On%20Success
      (Variables|/Script/UMG.TextBlock|SetText (Variables|/Game/Widgets/networkStats.networkStats_C|Gettxt_server_status (Variables|Default|GetNetworkStatsWidget)) "Online")
      (Variables|/Script/UMG.TextBlock|SetColorAndOpacity (Variables|/Game/Widgets/networkStats.networkStats_C|Gettxt_server_status (Variables|Default|GetNetworkStatsWidget)) (Utilities|Struct|MakeSlateColor "(R=0.292967,G=1.000000,B=0.245313,A=1.000000)" "UseColor_Specified"))
      (bind _outvalue (|GetJsonField _result_body "version"))
      (Widget|SetVisibility (Variables|/Game/Widgets/networkStats.networkStats_C|Gettxt_server_version (Variables|Default|GetNetworkStatsWidget)) "Visible")
      (Variables|/Script/UMG.TextBlock|SetText (Variables|/Game/Widgets/networkStats.networkStats_C|Gettxt_server_version (Variables|Default|GetNetworkStatsWidget)) _outvalue)
      (bind _returnvalue_2 (Actor|GetActorOfClass "/Game/Blueprints/bp_camera_controller.bp_camera_controller_C"))
      (if (Pawn|IsPlayerControlled _returnvalue_2)
        (bind _returnvalue_3 (UserInterface|CreateWidget "/Game/Widgets/agentRegisterWidget.agentRegisterWidget_C"))
        (UserInterface|Viewport|AddtoViewport _returnvalue_3 0)))
    (:On%20Error
      (Variables|/Script/UMG.TextBlock|SetText (Variables|/Game/Widgets/networkStats.networkStats_C|Gettxt_server_status (Variables|Default|GetNetworkStatsWidget)) "Offline")
      (Variables|/Script/UMG.TextBlock|SetColorAndOpacity (Variables|/Game/Widgets/networkStats.networkStats_C|Gettxt_server_status (Variables|Default|GetNetworkStatsWidget)) (Utilities|Struct|MakeSlateColor "(R=1.000000,G=0.195929,B=0.166081,A=1.000000)" "UseColor_Specified")))))

(fn ConstructionScript)